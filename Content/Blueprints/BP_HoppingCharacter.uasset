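; Player character for a Crossy Road-style endless hopper, moved on WASD in timeline-lerped 100-unit hops, one at a time.
; Backward hops are capped by MaxBack, which forward hops win back.
; BeginPlay spawns a random first section; Tick scores X distance from start.
; Zero health or an AFK timer, reset only by forward hops, opens Menu; starting-truck spawn loops are disconnected.
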(event `Key|W`
  (params (Key :type "Key Structure"))
  (bind _movevector (`self.MoveVector`))
  ;[1 1 1] Forward
  (:`Pressed`
    (if (and (`self.LeftTimerFinish`) (`self.BackwardsTimerFinish`) (`self.RightTimerFinish`))
      (if (`self.ForwardTimerFinished`)
        (set `self.AFKTimer` 10.0)
        (`|ExecutionSequence`
          (:`then_0`
            ;[1 1 1] Backwards Movement
            (if (<= (`self.MaxBack`) 3)
              (if (> (`self.MaxBack`) 0)
                (set `self.MaxBack` (- (`self.MaxBack`) 1)))))
          (:`then_1`
            (set `self.MoveVector` (`self.K2_GetActorLocation`))
            (set `self.ForwardTimerFinished` false)
            (bind (_direction _movement) (`Timeline|Timeline` :!via `PlayFromStart`)
              (:`Update`
                (bind _output_get (set `self.NewMoveVector` (`KismetMathLibrary.VLerp` _movevector (+ _movevector (100.0 0.0 0.0)) _movement)))
                (`self.K2_SetActorLocation` _output_get))
              (:`Finished`
                (`KismetSystemLibrary.DelayUntilNextTick`)
                (set `self.ForwardTimerFinished` true)))))))))

(event `Key|S`
  (params (Key :type "Key Structure"))
  (bind _movevector (`self.MoveVector`))
  ;[1 1 1] Backwards
  (:`Pressed`
    (if (and (`self.LeftTimerFinish`) (`self.ForwardTimerFinished`) (`self.RightTimerFinish`))
      (if (`self.BackwardsTimerFinish`)
        (if (< (`self.MaxBack`) 3)
          (set `self.MaxBack` (+ (`self.MaxBack`) 1))
          (set `self.MoveVector` (`self.K2_GetActorLocation`))
          (set `self.BackwardsTimerFinish` false)
          (bind (_direction _movement) (`Timeline|Timeline_0` :!via `PlayFromStart`)
            (:`Update`
              (`self.K2_SetActorLocation` (`KismetMathLibrary.VLerp` _movevector (+ _movevector (-100.0 0.0 0.0)) _movement)))
            (:`Finished`
              (`KismetSystemLibrary.DelayUntilNextTick`)
              (set `self.BackwardsTimerFinish` true))))))))

(event `Key|D`
  (params (Key :type "Key Structure"))
  (bind _movevector (`self.MoveVector`))
  ;[1 1 1] Right
  (:`Pressed`
    (if (and (`self.LeftTimerFinish`) (`self.ForwardTimerFinished`) (`self.BackwardsTimerFinish`))
      (if (`self.RightTimerFinish`)
        (set `self.MoveVector` (`self.K2_GetActorLocation`))
        (set `self.RightTimerFinish` false)
        (bind (_direction _movement) (`Timeline|Timeline_1` :!via `PlayFromStart`)
          (:`Update`
            (`self.K2_SetActorLocation` (`KismetMathLibrary.VLerp` _movevector (+ _movevector (0.0 100.0 0.0)) _movement)))
          (:`Finished`
            (`KismetSystemLibrary.DelayUntilNextTick`)
            (set `self.RightTimerFinish` true)))))))

(event `Key|A`
  (params (Key :type "Key Structure"))
  (bind _movevector (`self.MoveVector`))
  ;[1 1 1] Left
  (:`Pressed`
    (if (and (`self.RightTimerFinish`) (`self.ForwardTimerFinished`) (`self.BackwardsTimerFinish`))
      (if (`self.LeftTimerFinish`)
        (set `self.MoveVector` (`self.K2_GetActorLocation`))
        (set `self.LeftTimerFinish` false)
        (bind (_direction _movement) (`Timeline|Timeline_2` :!via `PlayFromStart`)
          (:`Update`
            (`self.K2_SetActorLocation` (`KismetMathLibrary.VLerp` _movevector (+ _movevector (0.0 -100.0 0.0)) _movement)))
          (:`Finished`
            (`KismetSystemLibrary.DelayUntilNextTick`)
            (set `self.LeftTimerFinish` true)))))))

(event `self.ReceiveAnyDamage`
  (params (Damage :type "Float (single-precision)") (DamageType :type "DamageType Object Reference") (InstigatedBy :type "Controller Object Reference") (DamageCauser :type "Actor Object Reference"))
  ;[1 1 1] Health
  (set `self.CurrentHealth` (`KismetMathLibrary.FTrunc` (- (`self.CurrentHealth`) Damage)))
  (if (<= (`self.CurrentHealth`) 0)
    (`GameplayStatics.OpenLevelBySoftObjectPtr` "/Game/Menu.Menu")))

(event `self.ReceiveBeginPlay`
  ;[1 1 1] Begin Play
  (`|ExecutionSequence`
    (:`then_0`
      (set `self.CharacterStart` (`self.K2_GetActorLocation`)))
    (:`then_1`
      (set `self.CurrentHealth` (`self.StartHealth`)))
    (:`then_2`
      (set `self.Score` (`self.Start Score`)))
    (:`then_3`
      (set `self.MaxBack` 0))
    (:`then_5`
      (bind _returnvalue (`GameplayStatics.GetActorOfClass` "/Game/BP_StartSection_.BP_StartSection__C")))
    (:`then_6`
      (set `self.Randomizer` (`KismetMathLibrary.RandomIntegerInRange` 0 4))
      (`|ExecutionSequence`
        (:`then_0`
          (if (== (`self.Randomizer`) 0)
            (`KismetSystemLibrary.PrintString` "1")
            (bind _returnvalue_2 (`KismetMathLibrary.MakeTransform` (+ (`self.K2_GetActorLocation` _returnvalue) (1000.0 0.0 0.0))))
            (bind _returnvalue_3 (`|SpawnActorFromClass` "/Game/BP_Section1.BP_Section1_C" _returnvalue_2 "Undefined" "MultiplyWithRoot" null null))
            (`/Game/BP_Section1.SectionSpawn` _returnvalue_3)))
        (:`then_1`
          (if (== (`self.Randomizer`) 1)
            (`KismetSystemLibrary.PrintString` "2")
            (bind _returnvalue_4 (`|SpawnActorFromClass` "/Game/BP_Section2.BP_Section2_C" _returnvalue_2 "Undefined" "MultiplyWithRoot" null null))
            (`/Game/BP_Section2.SectionSpawn` _returnvalue_4)))
        (:`then_2`
          (if (== (`self.Randomizer`) 2)
            (`KismetSystemLibrary.PrintString` "3")
            (bind _returnvalue_5 (`|SpawnActorFromClass` "/Game/BP_Section3.BP_Section3_C" _returnvalue_2 "Undefined" "MultiplyWithRoot" null null))
            (`/Game/BP_Section3.SpawnSection` _returnvalue_5)))
        (:`then_3`
          (if (== (`self.Randomizer`) 3)
            (`KismetSystemLibrary.PrintString` "4")
            (bind _returnvalue_6 (`|SpawnActorFromClass` "/Game/BP_Section4.BP_Section4_C" _returnvalue_2 "Undefined" "MultiplyWithRoot" null null))
            (`/Game/BP_Section4.SectionSpawn` _returnvalue_6)))
        (:`then_4`
          (if (== (`self.Randomizer`) 4)
            (`KismetSystemLibrary.PrintString` "5")
            (bind _returnvalue_7 (`|SpawnActorFromClass` "/Game/BP_Section5_.BP_Section5__C" _returnvalue_2 "Undefined" "MultiplyWithRoot" null null))
            (`/Game/BP_Section5_.SpawnSection` _returnvalue_7)))))))

(event `self.ReceiveTick`
  (params (DeltaSeconds :type "Float (single-precision)"))
  (bind _characterstart_x (`KismetMathLibrary.BreakVector` (`self.CharacterStart`)))
  ;[1 1 1] Score
  (`|ExecutionSequence`
    (:`then_0`
      (bind _output_get (set `self.Character Location` (`self.K2_GetActorLocation`)))
      (set `self.Score` (`KismetMathLibrary.Conv_Int64ToInt` (`KismetMathLibrary.FTrunc64` (/ (- (.x _output_get) _characterstart_x) 100.0)))))
    (:`then_1`
      (set `self.AFKTimer` (- (`self.AFKTimer`) DeltaSeconds))
      (if (<= (`self.AFKTimer`) 0.0)
        (`GameplayStatics.OpenLevelBySoftObjectPtr` "/Game/Menu.Menu")))))

(fn `UserConstructionScript`)