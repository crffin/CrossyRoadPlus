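; Trigger box that spawns the next random level section ahead when the hopping character enters it.
; On Box overlap by a BP_HoppingCharacter, a random integer selects one of five section Blueprints through a Sequence of equality checks.
; The chosen section spawns at a fixed offset from the trigger's location, then has its section-spawn call invoked.
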(event `self.Box.OnComponentBeginOverlap`
  (params (OverlappedComponent :type "PrimitiveComponent Object Reference") (OtherActor :type "Actor Object Reference") (OtherComp :type "PrimitiveComponent Object Reference") (OtherBodyIndex :type Integer) (bFromSweep :type Boolean) (SweepResult :type "HitResult Structure (by ref)"))
  (bind _returnvalue (`KismetMathLibrary.MakeTransform` (+ (`self.K2_GetActorLocation`) (2000.0 -200.0 0.0))))
  (if (`KismetMathLibrary.ClassIsChildOf` (`GameplayStatics.GetObjectClass` OtherActor) "/Game/Blueprints/BP_HoppingCharacter.BP_HoppingCharacter_C")
    (set `self.Randomizer` (`KismetMathLibrary.RandomIntegerInRange` 0 4))
    (`|ExecutionSequence`
      (:`then_0`
        (if (== (`self.Randomizer`) 0)
          (bind _returnvalue_2 (`|SpawnActorFromClass` "/Game/BP_Section1.BP_Section1_C" _returnvalue "Undefined" "MultiplyWithRoot" null null))
          (`/Game/BP_Section1.SectionSpawn` _returnvalue_2)))
      (:`then_1`
        (if (== (`self.Randomizer`) 1)
          (bind _returnvalue_3 (`|SpawnActorFromClass` "/Game/BP_Section2.BP_Section2_C" _returnvalue "Undefined" "MultiplyWithRoot" null null))
          (`/Game/BP_Section2.SectionSpawn` _returnvalue_3)))
      (:`then_2`
        (if (== (`self.Randomizer`) 2)
          (bind _returnvalue_4 (`|SpawnActorFromClass` "/Game/BP_Section3.BP_Section3_C" _returnvalue "Undefined" "MultiplyWithRoot" null null))
          (`/Game/BP_Section3.SpawnSection` _returnvalue_4)))
      (:`then_3`
        (if (== (`self.Randomizer`) 3)
          (bind _returnvalue_5 (`|SpawnActorFromClass` "/Game/BP_Section4.BP_Section4_C" _returnvalue "Undefined" "MultiplyWithRoot" null null))
          (`/Game/BP_Section4.SectionSpawn` _returnvalue_5)))
      (:`then_4`
        (if (== (`self.Randomizer`) 4)
          (bind _returnvalue_6 (`|SpawnActorFromClass` "/Game/BP_Section5_.BP_Section5__C" _returnvalue "Undefined" "MultiplyWithRoot" null null))
          (`/Game/BP_Section5_.SpawnSection` _returnvalue_6))))))

(fn `NewFunction`)

(fn `UserConstructionScript`)